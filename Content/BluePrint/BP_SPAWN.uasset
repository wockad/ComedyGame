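; BP_SPAWN is a spawner actor that keeps producing waves of BP_Charger actors.
; On BeginPlay it spawns one at each of its four spawn-point components, then loops through a five-second retriggerable delay to repeat indefinitely.
; A Destoryspawn event destroys the spawner.
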(event `self.ReceiveBeginPlay`
  (`|ExecutionSequence` :!label _label
    (:`then_0`
      (`|SpawnActorFromClass` "/Game/BluePrint/BP_Charger.BP_Charger_C" (`SceneComponent.K2_GetComponentToWorld` (`self.spawn1`)) "Undefined" "OverrideRootScale" null null))
    (:`then_1`
      (`|SpawnActorFromClass` "/Game/BluePrint/BP_Charger.BP_Charger_C" (`SceneComponent.K2_GetComponentToWorld` (`self.spawn2`)) "Undefined" "OverrideRootScale" null null))
    (:`then_2`
      (`|SpawnActorFromClass` "/Game/BluePrint/BP_Charger.BP_Charger_C" (`SceneComponent.K2_GetComponentToWorld` (`self.spawn3`)) "Undefined" "OverrideRootScale" null null))
    (:`then_3`
      (`|SpawnActorFromClass` "/Game/BluePrint/BP_Charger.BP_Charger_C" (`SceneComponent.K2_GetComponentToWorld` (`self.spawn4`)) "Undefined" "OverrideRootScale" null null))
    (:`then_4`
      (`KismetSystemLibrary.RetriggerableDelay` 5.0)
      (goto _label))))

(event `Destoryspawn`
  (`self.K2_DestroyActor`))

(fn `UserConstructionScript`)