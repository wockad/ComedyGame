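; BP_FP_Runner_GameMode is a game mode, apparently for a first-person runner, that keeps a countdown timer.
; BeginPlay sets Seconds to 30, and Tick feeds a one-second Delay that decrements it about once per second.
; A check that would reopen the current level at zero is unconnected, so it never runs and the count continues below zero.
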(event `self.ReceiveBeginPlay`
  (set `self.Seconds` 30))

(event `self.ReceiveTick`
  (params (DeltaSeconds :type "Float (single-precision)"))
  (`KismetSystemLibrary.Delay` 1.0)
  (set `self.Seconds` (- (`self.Seconds`) 1)))

(fn `UserConstructionScript`)