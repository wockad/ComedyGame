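; BP_AwesomePlatform is a damage-activated actor that shifts two platforms between preset positions.
; When damaged while idle, it swaps materials on both platforms and the rock and spawns a dust burst.
; A Sequence starts both eased moves together, each using a FlipFlop to alternate destinations on successive hits.
; IsMoving blocks retriggering until a move completes, when the materials switch again to their resting look.
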(event `self.ReceiveAnyDamage`
  (params (Damage :type "Float (single-precision)") (DamageType :type "DamageType Object Reference") (InstigatedBy :type "Controller Object Reference") (DamageCauser :type "Actor Object Reference"))
  (bind _platform (`self.Platform`))
  (bind _platform2 (`self.Platform2`))
  (if (not (`self.IsMoving`))
    (`PrimitiveComponent.SetMaterial` (`self.Platform`) 0 "/Game/My_Mats/MovingPlatform_Emi.MovingPlatform_Emi")
    (`PrimitiveComponent.SetMaterial` (`self.Platform2`) 0 "/Game/My_Mats/MovingPlatform_Emi.MovingPlatform_Emi")
    (`PrimitiveComponent.SetMaterial` (`self.Rock`) 0 "/Game/My_Mats/Emissive_Master_Inst.Emissive_Master_Inst")
    (`GameplayStatics.SpawnEmitterAtLocation` "/Game/StarterContent/Particles/P_Ambient_DustEXPLOSION_MovingPlatform.P_Ambient_DustEXPLOSION_MovingPlatform" (`SceneComponent.K2_GetComponentLocation` (`self.ParticleSpawn`)))
    (`|ExecutionSequence`
      (:`then_0`
        (set `self.IsMoving` true)
        (`/Engine/EditorBlueprintResources/StandardMacros.FlipFlop`
          (:`A`
            (`KismetSystemLibrary.MoveComponentTo` _platform (`self.Movloc1`) (struct) true true 3.0)
            (set `self.IsMoving` false))
          (:`B`
            (`KismetSystemLibrary.MoveComponentTo` _platform (`self.Movloc2`) (struct) true true 3.0)
            (set `self.IsMoving` false))))
      (:`then_1`
        (set `self.IsMoving` true)
        (`/Engine/EditorBlueprintResources/StandardMacros.FlipFlop`
          (:`A`
            (`KismetSystemLibrary.MoveComponentTo` _platform2 (`self.Movloc4`) (struct) true true 3.0)
            (set `self.IsMoving` false))
          (:`B`
            (`KismetSystemLibrary.MoveComponentTo` _platform2 (`self.Movloc3`) (struct) true true 3.0)
            (set `self.IsMoving` false)))))
    (`PrimitiveComponent.SetMaterial` (`self.Rock`) 0 "/Game/My_Mats/MovingPlatform_Emi.MovingPlatform_Emi")
    (`PrimitiveComponent.SetMaterial` (`self.Platform`) 0 "/Game/My_Mats/Brown.Brown")
    (`PrimitiveComponent.SetMaterial` (`self.Platform2`) 0 "/Game/My_Mats/Brown.Brown")))

(fn `UserConstructionScript`)