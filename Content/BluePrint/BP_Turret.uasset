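; BP_Turret is an enemy turret that turns toward the BP_FP_Runner player when PawnSensing sees it and fires BP_Charger actors.
; Each sighting updates its facing, while a boolean gate and Delay nodes space out spawns from a scene component.
; Any damage destroys it with a dust explosion, calls AddCrossHair on the runner cached at BeginPlay, and plays a camera shake at the player.
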(event `self.ReceiveBeginPlay`
  (bind _outactors (`GameplayStatics.GetAllActorsOfClass` "/Game/BluePrint/BP_FP_Runner.BP_FP_Runner_C"))
  (set `self.Player` (`|GetArrayItem` _outactors))
  (set `self.spawnprojectile` true))

(event `self.ReceiveAnyDamage`
  (params (Damage :type "Float (single-precision)") (DamageType :type "DamageType Object Reference") (InstigatedBy :type "Controller Object Reference") (DamageCauser :type "Actor Object Reference"))
  (`|ExecutionSequence`
    (:`then_0`
      (`GameplayStatics.SpawnEmitterAtLocation` "/Game/StarterContent/Particles/P_Ambient_DustEXPLOSION.P_Ambient_DustEXPLOSION" (`SceneComponent.K2_GetComponentLocation` (`self.Scene1`)))
      (`self.K2_DestroyActor`))
    (:`then_1`
      (`/Game/BluePrint/BP_FP_Runner.AddCrossHair` (`self.Player`)))
    (:`then_2`
      (`GameplayStatics.PlayWorldCameraShake` "/Game/BluePrint/BP_CameraShake_Fire.BP_CameraShake_Fire_C" (`self.K2_GetActorLocation` (`GameplayStatics.GetPlayerCharacter` 0)) 0.0 500.0))))

(event `self.PawnSensing.OnSeePawn`
  (params (Pawn :type "Pawn Object Reference"))
  (bind (_returnvalue_location _returnvalue_rotation) (`KismetMathLibrary.BreakTransform` (`SceneComponent.K2_GetComponentToWorld` (`self.Scene`))))
  (bind _asbp_fp_runner (cast `/Game/BluePrint/BP_FP_Runner` Pawn))
  (`|ExecutionSequence`
    (:`then_0`
      (`self.K2_SetActorRotation` (`KismetMathLibrary.FindLookAtRotation` (`self.K2_GetActorLocation`) (`self.K2_GetActorLocation` _asbp_fp_runner))))
    (:`then_1`
      (if (`self.spawnprojectile`)
        (`KismetSystemLibrary.Delay` 2.0)
        (`|SpawnActorFromClass` "/Game/BluePrint/BP_Charger.BP_Charger_C" (`KismetMathLibrary.MakeTransform` _returnvalue_location _returnvalue_rotation) "Undefined" "OverrideRootScale" null null)
        (set `self.spawnprojectile` false)
        (`KismetSystemLibrary.Delay` 3.0)
        (set `self.spawnprojectile` true)))))

(fn `UserConstructionScript`)