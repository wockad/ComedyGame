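; Thrown dagger projectile for the first-person runner that damages enemies, crystals and moving platforms, then self-destructs after a timeout.
; A self-restarting timeline spins the mesh until the first box hit stops it and its particles.
; Box overlap handles Chargers, while Hit uses a cast chain for crystals, platforms and spawners, also decrementing spawner health directly.
; Charger, crystal and spawner hits increment GameMode Seconds; crystals also call AddCrossHair.
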(event `self.Box.OnComponentHit`
  (params (HitComponent :type "PrimitiveComponent Object Reference") (OtherActor :type "Actor Object Reference") (OtherComp :type "PrimitiveComponent Object Reference") (NormalImpulse :type "Vector Structure") (Hit :type "HitResult Structure (by ref)"))
  ;[1 1 1] Stop Rotation and deactivate particle system on hit
  (`/Engine/EditorBlueprintResources/StandardMacros.DoOnce` false
    (:`Completed`
      (`ActorComponent.Deactivate` (`self.ParticleSystem`))
      (`self.Stoprotate`))))

(event `OnSwordRotate`
  (bind _dagger (`self.Dagger`))
  (bind (_returnvalue_roll _returnvalue_pitch _returnvalue_yaw) (`KismetMathLibrary.BreakRotator` (`SceneComponent.K2_GetComponentRotation` _dagger)))
  ;[1 1 1] Rotate Dagger manager
  (bind (_direction _newtrack_0) (`Timeline|SwordRotate` :!label _label)
    (:`Update`
      (`SceneComponent.K2_SetWorldRotation` _dagger (`KismetMathLibrary.MakeRotator` (`KismetMathLibrary.Lerp` 0.0 360.0 _newtrack_0) _returnvalue_pitch _returnvalue_yaw) false false))
    (:`Finished`
      (`self.OnSwordRotate`))))

(event `Stoprotate`
  ;[1 1 1] Rotate Dagger manager
  (goto _label :!via `Stop`))

(event `self.ReceiveBeginPlay`
  ;[1 1 1] Set rotation speed and destroy actor
  (`TimelineComponent.SetPlayRate` (`self.SwordRotate`) (/ 1.0 (`self.SwordRotation`)))
  (`self.OnSwordRotate`)
  (`KismetSystemLibrary.Delay` 60.0)
  (`self.K2_DestroyActor`))

(event `self.Box.OnComponentBeginOverlap`
  (params (OverlappedComponent :type "PrimitiveComponent Object Reference") (OtherActor :type "Actor Object Reference") (OtherComp :type "PrimitiveComponent Object Reference") (OtherBodyIndex :type Integer) (bFromSweep :type Boolean) (SweepResult :type "HitResult Structure (by ref)"))
  ;[1 1 1] Enemy hit manager
  (bind _asbp_charger (cast `/Game/BluePrint/BP_Charger` OtherActor))
  (`GameplayStatics.ApplyDamage` _asbp_charger 1.0 null self)
  (bind _asbp_fp_runner_game_mode (cast `/Game/BluePrint/BP_FP_Runner_GameMode` (`GameplayStatics.GetGameMode`)))
  (set `/Game/BluePrint/BP_FP_Runner_GameMode.Seconds` (+ (`/Game/BluePrint/BP_FP_Runner_GameMode.Seconds` _asbp_fp_runner_game_mode) 1) _asbp_fp_runner_game_mode)
  (`self.K2_DestroyActor`))

(event `self.ReceiveHit`
  (params (MyComp :type "PrimitiveComponent Object Reference") (Other :type "Actor Object Reference") (OtherComp :type "PrimitiveComponent Object Reference") (bSelfMoved :type Boolean) (HitLocation :type "Vector Structure") (HitNormal :type "Vector Structure") (NormalImpulse :type "Vector Structure") (Hit :type "HitResult Structure (by ref)"))
  ;[1 1 1] Crystal hit manager
  (`|ExecutionSequence`
    (:`then_0`
      (bind _asbp_crystal_01 (cast `/Game/BluePrint/Crystals/BP_Crystal_01` Other))
      (`GameplayStatics.ApplyDamage` _asbp_crystal_01 1.0)
      (bind _asbp_fp_runner (cast `/Game/BluePrint/BP_FP_Runner` (`GameplayStatics.GetPlayerCharacter` 0)))
      (`/Game/BluePrint/BP_FP_Runner.AddCrossHair` _asbp_fp_runner)
      (bind _asbp_fp_runner_game_mode (cast `/Game/BluePrint/BP_FP_Runner_GameMode` (`GameplayStatics.GetGameMode`)))
      (set `/Game/BluePrint/BP_FP_Runner_GameMode.Seconds` (+ (`/Game/BluePrint/BP_FP_Runner_GameMode.Seconds` _asbp_fp_runner_game_mode) 1) _asbp_fp_runner_game_mode)
      (`self.K2_DestroyActor`))
    (:`then_1`
      (bind _asbp_crystal_02 (cast `/Game/BluePrint/Crystals/BP_Crystal_02` Other))
      (`GameplayStatics.ApplyDamage` _asbp_crystal_02 1.0)
      (bind _asbp_fp_runner_2 (cast `/Game/BluePrint/BP_FP_Runner` (`GameplayStatics.GetPlayerCharacter` 0)))
      (`/Game/BluePrint/BP_FP_Runner.AddCrossHair` _asbp_fp_runner_2)
      (bind _asbp_fp_runner_game_mode_2 (cast `/Game/BluePrint/BP_FP_Runner_GameMode` (`GameplayStatics.GetGameMode`)))
      (set `/Game/BluePrint/BP_FP_Runner_GameMode.Seconds` (+ (`/Game/BluePrint/BP_FP_Runner_GameMode.Seconds` _asbp_fp_runner_game_mode_2) 1) _asbp_fp_runner_game_mode_2)
      (`self.K2_DestroyActor`))
    (:`then_2`
      (bind _asbp_crystal_03 (cast `/Game/BluePrint/Crystals/BP_Crystal_03` Other))
      (`GameplayStatics.ApplyDamage` _asbp_crystal_03 1.0)
      (bind _asbp_fp_runner_3 (cast `/Game/BluePrint/BP_FP_Runner` (`GameplayStatics.GetPlayerCharacter` 0)))
      (`/Game/BluePrint/BP_FP_Runner.AddCrossHair` _asbp_fp_runner_3)
      (bind _asbp_fp_runner_game_mode_3 (cast `/Game/BluePrint/BP_FP_Runner_GameMode` (`GameplayStatics.GetGameMode`)))
      (set `/Game/BluePrint/BP_FP_Runner_GameMode.Seconds` (+ (`/Game/BluePrint/BP_FP_Runner_GameMode.Seconds` _asbp_fp_runner_game_mode_3) 1) _asbp_fp_runner_game_mode_3)
      (`self.K2_DestroyActor`))
    (:`then_3`
      (bind _asbp_crystal_04 (cast `/Game/BluePrint/Crystals/BP_Crystal_04` Other))
      (`GameplayStatics.ApplyDamage` _asbp_crystal_04 1.0)
      (bind _asbp_fp_runner_4 (cast `/Game/BluePrint/BP_FP_Runner` (`GameplayStatics.GetPlayerCharacter` 0)))
      (`/Game/BluePrint/BP_FP_Runner.AddCrossHair` _asbp_fp_runner_4)
      (bind _asbp_fp_runner_game_mode_4 (cast `/Game/BluePrint/BP_FP_Runner_GameMode` (`GameplayStatics.GetGameMode`)))
      (set `/Game/BluePrint/BP_FP_Runner_GameMode.Seconds` (+ (`/Game/BluePrint/BP_FP_Runner_GameMode.Seconds` _asbp_fp_runner_game_mode_4) 1) _asbp_fp_runner_game_mode_4)
      (`self.K2_DestroyActor`))
    (:`then_4`
      (bind _asbp_moving_platform (cast `/Game/BluePrint/Bp_MovingPlatform` Other))
      (`GameplayStatics.ApplyDamage` (`ActorComponent.GetOwner` (`/Game/BluePrint/Bp_MovingPlatform.Rock` _asbp_moving_platform)) 1.0))
    (:`then_5`
      ;[1 1 1] Deal damage to spawner enemy
      (bind _asbp_spawner (cast `/Game/BluePrint/BP_Spawner` Other))
      (set `/Game/BluePrint/BP_Spawner.Current health` (- (`/Game/BluePrint/BP_Spawner.Current health` _asbp_spawner) 1.0) _asbp_spawner)
      (`/Engine/EditorBlueprintResources/StandardMacros.DoOnce` false
        (:`Completed`
          (`GameplayStatics.ApplyDamage` _asbp_spawner 1.0)
          (bind _asbp_fp_runner_game_mode_5 (cast `/Game/BluePrint/BP_FP_Runner_GameMode` (`GameplayStatics.GetGameMode`)))
          (set `/Game/BluePrint/BP_FP_Runner_GameMode.Seconds` (+ (`/Game/BluePrint/BP_FP_Runner_GameMode.Seconds` _asbp_fp_runner_game_mode_5) 1) _asbp_fp_runner_game_mode_5))))))

(fn `UserConstructionScript`)