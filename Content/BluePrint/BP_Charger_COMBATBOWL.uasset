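; Charger enemy with a spinning blade body that hunts BP_FP_Runner and restarts the current level when its sphere touches the player.
; Pawn sensing triggers aggro, after which Tick keeps issuing move orders, facing and spinning.
; Sightings also start a timed attack: stop, hop with a slower spin, then launch at the player spinning faster.
; Any damage kills it instantly with crosshair feedback, a dust explosion and camera shake.
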(event `self.ReceiveAnyDamage`
  (params (Damage :type "Float (single-precision)") (DamageType :type "DamageType Object Reference") (InstigatedBy :type "Controller Object Reference") (DamageCauser :type "Actor Object Reference"))
  ;[1 1 1] Death
  (set `self.Isalive` false)
  (`|ExecutionSequence`
    (:`then_0`
      ;;[1 0 0] Apply damage crosshair
      (`/Game/BluePrint/BP_FP_Runner.AddCrossHair` (`self.Player`)))
    (:`then_1`
      ;;[1 1 1] Spawn particles and destroy actory
      (`GameplayStatics.SpawnEmitterAtLocation` "/Game/StarterContent/Particles/P_Ambient_DustEXPLOSION.P_Ambient_DustEXPLOSION" (`SceneComponent.K2_GetComponentLocation` (`self.Scene`)))
      (`self.K2_DestroyActor`))
    (:`then_2`
      ;;[1 1 1] Apply camerashake
      (`GameplayStatics.PlayWorldCameraShake` "/Game/BluePrint/BP_CameraShake_Fire.BP_CameraShake_Fire_C" (`self.K2_GetActorLocation` (`GameplayStatics.GetPlayerCharacter` 0)) 0.0 500.0))))

(event `self.ReceiveBeginPlay`
  ;[1 1 1] Set up player refrence and set alive
  (set `self.Isalive` true)
  (bind _outactors (`GameplayStatics.GetAllActorsOfClass` "/Game/BluePrint/BP_FP_Runner.BP_FP_Runner_C"))
  (set `self.Player` (`|GetArrayItem` _outactors)))

(event `self.PawnSensing.OnSeePawn`
  (params (Pawn :type "Pawn Object Reference"))
  (bind _returnvalue (`self.K2_GetActorLocation` (`GameplayStatics.GetPlayerCharacter` 0)))
  ;[1 1 1] Move towards player
  (`self.RotateBlade`)
  (bind _asbp_fp_runner (cast `/Game/BluePrint/BP_FP_Runner` Pawn))
  (`|ExecutionSequence`
    (:`then_0`
      (`|AIMoveTo` self _returnvalue _asbp_fp_runner
        (:`then`
          (`AIBlueprintHelperLibrary.SimpleMoveToLocation` null _returnvalue))))
    (:`then_1`
      (bind _returnvalue_2 (`KismetMathLibrary.FindLookAtRotation` (`self.K2_GetActorLocation`) (`self.K2_GetActorLocation` _asbp_fp_runner)))
      ;[1 1 1] Set rotation towards player
      (`self.K2_SetActorRotation` _returnvalue_2)
      (set `self.AggroActive` true))
    (:`then_2`
      ;[1 1 1] Fly towards player
      (if (`self.Isalive`)
        (if (`self.ShouldFly`)
          (`MovementComponent.StopMovementImmediately` (`self.CharacterMovement`))
          (set `self.ShouldFly` false)
          (set `self.RotationSpeed` 5.0)
          (`self.LaunchCharacter` (0.0 0.0 100.0) true)
          (`KismetSystemLibrary.Delay` 1.0)
          (set `self.RotationSpeed` 15.0)
          (`self.LaunchCharacter` (- (* (`KismetMathLibrary.GetForwardVector` _returnvalue_2) (`self.LaunchToPlayerForce`)) (0.0 0.0 100.0)))
          (`KismetSystemLibrary.Delay` 3.0)
          (`MovementComponent.StopMovementImmediately` (`self.CharacterMovement`))
          (set `self.ShouldFly` true))))))

(event `self.ReceiveTick`
  (params (DeltaSeconds :type "Float (single-precision)"))
  ;[1 1 1] update rotation and move to when aggro is true
  (if (`self.AggroActive`)
    (`|AIMoveTo` self (`self.K2_GetActorLocation` (`GameplayStatics.GetPlayerCharacter` 0)) null
      (:`then`
        (`self.K2_SetActorRotation` (`KismetMathLibrary.FindLookAtRotation` (`self.K2_GetActorLocation`) (`self.K2_GetActorLocation` (stale `self.PawnSensing.OnSeePawn` _asbp_fp_runner))))
        (`self.RotateBlade`)))))

(event `self.Sphere.OnComponentBeginOverlap`
  (params (OverlappedComponent :type "PrimitiveComponent Object Reference") (OtherActor :type "Actor Object Reference") (OtherComp :type "PrimitiveComponent Object Reference") (OtherBodyIndex :type Integer) (bFromSweep :type Boolean) (SweepResult :type "HitResult Structure (by ref)"))
  ;[1 1 1] Kill player open level
  (cast `/Game/BluePrint/BP_FP_Runner` OtherActor)
  (bind _returnvalue (`GameplayStatics.GetCurrentLevelName` true))
  (`GameplayStatics.OpenLevel` (`KismetStringLibrary.Conv_StringToName` _returnvalue)))

(event `RotateBlade`
  ;[1 1 1] Rotate Body
  (if (`self.AggroActive`)
    (if (`self.Isalive`)
      (`SceneComponent.K2_AddRelativeRotation` (`self.Body`) (`KismetMathLibrary.MakeRotator` 0.0 0.0 (`self.RotationSpeed`)) false false))))

(fn `UserConstructionScript`)